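; BP_LockedCase is an interactable case that brings up a password entry widget when the nearby player presses Interact.
; Its Box overlap events set IsPlayerClose and toggle actor input for player controller 0 as the FirstPersonCharacter enters or leaves.
; Each valid press creates a new WBP_PasswordUI; no unlock logic lives here.
; A debug counter prints on every begin overlap, whatever the actor.
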(event OnComponentEndOverlap(Box)
  (params (OverlappedComponent :type Primitive%20Component%20Object%20Reference) (OtherActor :type Actor%20Object%20Reference) (OtherComp :type Primitive%20Component%20Object%20Reference) (OtherBodyIndex :type Integer))
  (Utilities|Casting|CastToFirstPersonCharacter OtherActor)
  (Variables|Default|SetbIsPlayerClose false)
  (Input|DisableInput (Game|GetPlayerController 0)))

(event OnComponentBeginOverlap(Box)
  (params (OverlappedComponent :type Primitive%20Component%20Object%20Reference) (OtherActor :type Actor%20Object%20Reference) (OtherComp :type Primitive%20Component%20Object%20Reference) (OtherBodyIndex :type Integer) (bFromSweep :type Boolean) (SweepResult :type Hit%20Result%20Structure%20%28by%20ref%29))
  (Variables|Default|SetnumOverlap (+ (Variables|Default|GetnumOverlap) 1))
  (Development|PrintString (Utilities|String|ToString(Integer) (Variables|Default|GetnumOverlap)))
  (Utilities|Casting|CastToFirstPersonCharacter OtherActor)
  (Variables|Default|SetbIsPlayerClose true)
  (Input|EnableInput (Game|GetPlayerController 0)))

(event Input|ActionEvents|InputActionInteract
  (params (Key :type Key%20Structure :default "None"))
  (:Pressed
    (if (Variables|Default|GetbIsPlayerClose)
      (bind _returnvalue (UserInterface|CreateWidget "/Game/Blueprints/WBP_PasswordUI.WBP_PasswordUI_C"))
      (UserInterface|Viewport|AddtoViewport _returnvalue 0))))

(fn ConstructionScript)