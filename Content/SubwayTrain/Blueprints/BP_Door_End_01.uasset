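; End door in the subway train that the player swings open and closed with Interact, provided the character has a key.
; A box overlap tracks whether the first-person character is close and toggles input on the actor.
; A FlipFlop plays or reverses a timeline that sets the root's absolute world yaw.
; Overlap events print debug strings, including an overlap count read from LockedCase.
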(event OnComponentBeginOverlap(Box)
  (params (OverlappedComponent :type Primitive%20Component%20Object%20Reference) (OtherActor :type Actor%20Object%20Reference) (OtherComp :type Primitive%20Component%20Object%20Reference) (OtherBodyIndex :type Integer) (bFromSweep :type Boolean) (SweepResult :type Hit%20Result%20Structure%20%28by%20ref%29))
  (Development|PrintString (Utilities|String|ToString(Integer) (Variables|/Game/Blueprints/BP_LockedCase.BP_LockedCase_C|GetnumOverlap (Variables|Default|GetLockedCase))))
  (Utilities|Casting|CastToFirstPersonCharacter OtherActor)
  (Development|PrintString "Begin Overlap")
  (Variables|Default|SetbIsPlayerClose true)
  (Input|EnableInput (Game|GetPlayerController 0)))

(event OnComponentEndOverlap(Box)
  (params (OverlappedComponent :type Primitive%20Component%20Object%20Reference) (OtherActor :type Actor%20Object%20Reference) (OtherComp :type Primitive%20Component%20Object%20Reference) (OtherBodyIndex :type Integer))
  (Utilities|Casting|CastToFirstPersonCharacter OtherActor)
  (Development|PrintString "End Overlap")
  (Variables|Default|SetbIsPlayerClose false)
  (Input|DisableInput (Game|GetPlayerController 0)))

(event Input|ActionEvents|InputActionInteract
  (params (Key :type Key%20Structure :default "None"))
  (:Pressed
    (if (Variables|Default|GetbIsPlayerClose)
      (bind _asfirst_person_character (Utilities|Casting|CastToFirstPersonCharacter (Game|GetPlayerCharacter 0)))
      (if (Variables|/Game/FirstPersonBP/Blueprints/FirstPersonCharacter.FirstPersonCharacter_C|GetbHasKey _asfirst_person_character)
        (Utilities|FlowControl|FlipFlop
          (:A
            (bind _rotatedoor (Timeline|DoorTimeline Play)
              (:Update
                (Transformation|SetWorldRotation (Variables|Default|GetDefaultSceneRoot) (Math|Rotator|MakeRotator 0.0 0.0 _rotatedoor) false false))))
          (:B
            (Timeline|DoorTimeline Reverse)))))))

(fn ConstructionScript)